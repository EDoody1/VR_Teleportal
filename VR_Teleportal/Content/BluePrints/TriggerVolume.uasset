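; Trigger volume actor with a construction-sized box that fires its attached trigger handler components when a MotionControllerPawn_Portal overlaps it.
; BeginPlay caches the TriggerHandlerComponenet list, and each overlap calls Trigger on every entry.
; The volume's own Trigger event takes a handler and invokes its target function by name on its target actor through a timer.
; That event applies the handler's delay twice, as a Delay and as the timer time.
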(event OnComponentBeginOverlap(Box)
  (params (OverlappedComponent :type Primitive%20Component%20Object%20Reference) (OtherActor :type Actor%20Object%20Reference) (OtherComp :type Primitive%20Component%20Object%20Reference) (OtherBodyIndex :type Integer) (bFromSweep :type Boolean) (SweepResult :type Hit%20Result%20Structure%20%28by%20ref%29))
  (bind _triggerhandlers (Variables|Default|GetTriggerHandlers))
  (Utilities|Casting|CastToMotionControllerPawn_Portal OtherActor)
  (for (_array_element _array_index) _triggerhandlers
    (Development|PrintString (Utilities|GetDisplayName (Utilities|Array|Get(acopy) _triggerhandlers _array_index)))
    (Default|Trigger _array_element)))

(event Custom|Trigger
  (params (Handler :type Trigger%20Handler%20Componenet%20Object%20Reference))
  (bind _delay (Variables|/Game/BluePrints/TriggerHandlerComponenet.TriggerHandlerComponenet_C|GetDelay Handler))
  (bind _targetactor (Variables|/Game/BluePrints/TriggerHandlerComponenet.TriggerHandlerComponenet_C|GetTargetActor Handler))
  (bind _targetfunction (Variables|/Game/BluePrints/TriggerHandlerComponenet.TriggerHandlerComponenet_C|GetTargetFunction Handler))
  (Development|PrintString (Utilities|GetDisplayName _targetactor))
  (Development|PrintString _targetfunction)
  (Utilities|FlowControl|Delay _delay)
  (Utilities|Time|SetTimerbyFunctionName _targetactor _targetfunction _delay))

(event EventBeginPlay
  (Variables|Default|SetTriggerHandlers (Actor|GetComponentsByClass self "/Game/BluePrints/TriggerHandlerComponenet.TriggerHandlerComponenet_C"))
  (Utilities|IsValid (Variables|Default|GetTargetActorIN%20VOLUME)
    (:Is%20Not%20Valid
      (Variables|Default|SetTargetActorIN%20VOLUME self))))

(fn ConstructionScript
  (Components|Box|SetBoxExtent (Variables|Default|GetBox) (Math|Vector|MakeVector (Variables|Default|GetBoxX) (Variables|Default|GetBoxY) (Variables|Default|GetBoxZ)) true))

(fn Null)