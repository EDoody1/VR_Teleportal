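; Spawn point controller that teleports the MotionControllerPawn_Portal player to a chosen spawn position on BeginPlay.
; SpawnWhere selects one of six spawn references; an invalid one decrements the index and recursively retries lower slots, with no teleport if none is valid.
; The construction script caches the first pawn of that class as Player.
; If Player is invalid at teleport time, it is looked up again, but the teleport is not retried.
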(event Custom|Get%20player
  (bind _outactors (Actor|GetAllActorsOfClass "/Game/BluePrints/MotionControllerPawn_Portal.MotionControllerPawn_Portal_C"))
  (Variables|Default|SetPlayer (Utilities|Array|Get(acopy) _outactors)))

(event Custom|Teleport%20Player
  (bind _player (Variables|Default|GetPlayer))
  (bind _spawn_position_0 (Variables|Default|GetSpawn%20Position%200))
  (bind _spawn_position_1 (Variables|Default|GetSpawn%20Position%201))
  (bind _spawn_position_2 (Variables|Default|GetSpawn%20Position%202))
  (bind _spawn_position_3 (Variables|Default|GetSpawn%20Position%203))
  (bind _spawn_position_4 (Variables|Default|GetSpawn%20Position%204))
  (bind _spawn_position_5 (Variables|Default|GetSpawn%20Position%205))
  (Utilities|IsValid _player
    (:Is%20Valid
      (switch int (Variables|Default|GetSpawnWhere?)
        (:0
          (Utilities|IsValid _spawn_position_0
            (:Is%20Valid
              (Variables|Default|SetValidSpawnTarget _spawn_position_0)
              (Default|BasicTeleportEvent _player (Transformation|GetActorLocation (Variables|Default|GetValidSpawnTarget)) :!label _label))
            (:Is%20Not%20Valid
              (Variables|Default|SetSpawnWhere? (- (Variables|Default|GetSpawnWhere?) 1) :!label _label_2)
              (CallFunction|TeleportPlayer))))
        (:1
          (Utilities|IsValid _spawn_position_1
            (:Is%20Valid
              (Variables|Default|SetValidSpawnTarget _spawn_position_1)
              (goto _label))
            (:Is%20Not%20Valid
              (goto _label_2))))
        (:2
          (Utilities|IsValid _spawn_position_2
            (:Is%20Valid
              (Variables|Default|SetValidSpawnTarget _spawn_position_2)
              (goto _label))
            (:Is%20Not%20Valid
              (goto _label_2))))
        (:3
          (Utilities|IsValid _spawn_position_3
            (:Is%20Valid
              (Variables|Default|SetValidSpawnTarget _spawn_position_3)
              (goto _label))
            (:Is%20Not%20Valid
              (goto _label_2))))
        (:4
          (Utilities|IsValid _spawn_position_4
            (:Is%20Valid
              (Variables|Default|SetValidSpawnTarget _spawn_position_4)
              (goto _label))
            (:Is%20Not%20Valid
              (goto _label_2))))
        (:5
          (Utilities|IsValid _spawn_position_5
            (:Is%20Valid
              (Variables|Default|SetValidSpawnTarget _spawn_position_5)
              (goto _label))
            (:Is%20Not%20Valid
              (goto _label_2))))))
    (:Is%20Not%20Valid
      (CallFunction|GetPlayer))))

(event EventBeginPlay
  (CallFunction|TeleportPlayer))

(event Collision|EventActorBeginOverlap
  (params (OtherActor :type Actor%20Object%20Reference)))

(event EventTick
  (params (DeltaSeconds :type Float%20%28single-precision%29)))

(fn ConstructionScript
  (bind _outactors (Actor|GetAllActorsOfClass "/Game/BluePrints/MotionControllerPawn_Portal.MotionControllerPawn_Portal_C"))
  (Variables|Default|SetPlayer (Utilities|Array|Get(acopy) _outactors)))