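; One-shot physical VR push button that calls a named function on a target actor, defaulting to itself.
; Tick moves the button mesh with a physics-driven sphere within clamped travel until it crosses the press threshold.
; It then disables the spheres and constraint, eases the mesh to the pressed height and triggers the function via a short timer.
; A timeline crossfades two lights and the stand's material fades as feedback.
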(event OnComponentBeginOverlap(EnablingSphere)
  (params (OverlappedComponent :type Primitive%20Component%20Object%20Reference) (OtherActor :type Actor%20Object%20Reference) (OtherComp :type Primitive%20Component%20Object%20Reference) (OtherBodyIndex :type Integer) (bFromSweep :type Boolean) (SweepResult :type Hit%20Result%20Structure%20%28by%20ref%29)))

(event OnComponentEndOverlap(Mesh)
  (params (OverlappedComponent :type Primitive%20Component%20Object%20Reference) (OtherActor :type Actor%20Object%20Reference) (OtherComp :type Primitive%20Component%20Object%20Reference) (OtherBodyIndex :type Integer))
  (if (== OtherActor (Variables|Default|GetHittingObject))
    (Development|PrintString "Ended Overlap")
    (Utilities|FlowControl|Delay 0.2)
    (else
      (Development|PrintString "NON Hitting Object End Overlap"))))

(event OnComponentEndOverlap(EnablingSphere)
  (params (OverlappedComponent :type Primitive%20Component%20Object%20Reference) (OtherActor :type Actor%20Object%20Reference) (OtherComp :type Primitive%20Component%20Object%20Reference) (OtherBodyIndex :type Integer)))

(event Custom|Disable%20Physics
  (bind _sphere1 (Variables|Default|GetSphere1))
  (Physics|SetSimulatePhysics _sphere1 false)
  (Collision|SetCollisionEnabled _sphere1 "NoCollision")
  (Components|Activation|SetActive (Variables|Default|GetPhysicsConstraint) false false))

(event Custom|Press
  (Development|PrintString "PRESSED")
  (Utilities|Time|SetTimerbyFunctionName (Variables|Default|GetTargetActor) (Variables|Default|GetTargetFunction) 0.1)
  (CallFunction|AnimateMaterials))

(event Custom|Animate%20Materials
  (bind _sm_buttonstand (Variables|Default|GetSM_ButtonStand))
  (bind _newtrack_0 (Timeline|MaterialTimeline PlayFromStart)
    (:Update
      (Rendering|Components|Light|SetIntensity (Variables|Default|GetPointLight) (* _newtrack_0 5e+02))
      (Rendering|Components|Light|SetIntensity (Variables|Default|GetButtonLightRectLight) (- 5e+02 (* _newtrack_0 5e+02)))
      (Rendering|Material|SetScalarParameterValueonMaterials _sm_buttonstand "Right UV Fade" _newtrack_0)
      (Rendering|Material|SetScalarParameterValueonMaterials _sm_buttonstand "Left UV Fade" (- 1.0 _newtrack_0)))))

(event EventBeginPlay
  (Utilities|IsValid (Variables|Default|GetTargetActor)
    (:Is%20Valid
      _)
    (:Is%20Not%20Valid
      (Variables|Default|SetTargetActor self)))
  (Utilities|FlowControl|Delay 0.5)
  (Variables|Default|SetActive true))

(event EventTick
  (params (DeltaSeconds :type Float%20%28single-precision%29))
  (bind _sm_button (Variables|Default|GetSM_Button))
  (bind _sphere2 (Variables|Default|GetSphere2))
  (bind _sm_buttonstand (Variables|Default|GetSM_ButtonStand))
  (bind _returnvalue (Transformation|GetWorldLocation _sphere2))
  (bind _returnvalue_2 (Transformation|GetWorldLocation _sm_buttonstand))
  (bind _relativelocation (Variables|/Script/Engine.SceneComponent|GetRelativeLocation _sm_button))
  (bind _returnvalue_3 (- (.z _returnvalue) (.z _returnvalue_2)))
  (if (Variables|Default|GetActive)
    (Utilities|FlowControl|Sequence
      (:then_0
        (if (not (> (.z (Variables|/Script/Engine.SceneComponent|GetRelativeLocation (Variables|Default|GetSM_Button))) 165.0))
          (Variables|Default|SetPressed true)
          (CallFunction|DisablePhysics)
          (Utilities|FlowControl|DoOnce false
            (:Completed
              (CallFunction|Press)))))
      (:then_1
        (if (Variables|Default|GetPressed)
          (if (!= 165.0 (.z _relativelocation))
            (Transformation|SetRelativeLocation _sm_button (Math|Vector|MakeVector 0.0 0.0 (Math|Interpolation|FInterpTo (.z _relativelocation) 165.0 DeltaSeconds 1.0)) false false))
          (elif (!= _returnvalue_3 (.z (Variables|/Script/Engine.SceneComponent|GetRelativeLocation (Variables|Default|GetSM_Button))))
            (Transformation|SetRelativeLocation (Variables|Default|GetSM_Button) (Math|Vector|MakeVector 0.0 0.0 (Math|Float|Clamp(Float) _returnvalue_3 1.6e+02 175.0)) false false)))))))

(event Collision|EventHit
  (params (MyComp :type Primitive%20Component%20Object%20Reference) (Other :type Actor%20Object%20Reference) (OtherComp :type Primitive%20Component%20Object%20Reference) (bSelfMoved :type Boolean) (HitLocation :type Vector :default "0, 0, 0") (HitNormal :type Vector :default "0, 0, 0") (NormalImpulse :type Vector :default "0, 0, 0") (Hit :type Hit%20Result%20Structure%20%28by%20ref%29))
  (Variables|Default|SetHittingObject Other))

(fn ConstructionScript)