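; BP_CircleDoor is a door that opens and closes by rotating four hinge components together in yaw, up to 60 degrees.
; A single timeline drives the hinges, playing forward to open and in reverse to close, with play rate derived from separate open and close durations.
; When Looping is set, it alternates direction after a short pause.
; Open and Close functions trigger the motion; BeginPlay does nothing.
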(event Custom|CloseEvent
  (Components|Timeline|SetPlayRate (Variables|Default|GetTL_OpenClose) (/ 1.0 (Variables|Default|GetClose%20Duration)))
  (bind (_direction _newtrack_0) (Timeline|TL_OpenClose Reverse)
    (:Update
      (Transformation|SetRelativeRotation (Variables|Default|GetHinge1) (Math|Rotator|MakeRotator 0.0 0.0 (* _newtrack_0 6e+01)) false false))
    (:Finished
      (if (Variables|Default|GetLooping?)
        (switch Utilities|FlowControl|Switch|SwitchonETimelineDirection _direction
          (:Forward
            (Utilities|FlowControl|Delay 0.5)
            (CallFunction|CloseEvent))
          (:Backward
            (Utilities|FlowControl|Delay 0.5)
            (CallFunction|OpenEvent)))))))

(event Custom|OpenEvent
  (Components|Timeline|SetPlayRate (Variables|Default|GetTL_OpenClose) (/ 1.0 (Variables|Default|GetOpen%20Duration)))
  (bind (_direction _newtrack_0) (Timeline|TL_OpenClose Play)
    (:Update
      (Transformation|SetRelativeRotation (Variables|Default|GetHinge1) (Math|Rotator|MakeRotator 0.0 0.0 (* _newtrack_0 6e+01)) false false))
    (:Finished
      (if (Variables|Default|GetLooping?)
        (switch Utilities|FlowControl|Switch|SwitchonETimelineDirection _direction
          (:Forward
            (Utilities|FlowControl|Delay 0.5)
            (CallFunction|CloseEvent))
          (:Backward
            (Utilities|FlowControl|Delay 0.5)
            (CallFunction|OpenEvent)))))))

(event EventBeginPlay)

(fn ConstructionScript)

(fn Open
  (CallFunction|OpenEvent))

(fn Close
  (CallFunction|CloseEvent))