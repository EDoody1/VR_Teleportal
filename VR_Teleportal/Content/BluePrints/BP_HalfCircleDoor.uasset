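; BP_HalfCircleDoor is a two-part sliding door that opens and closes through its Open and Close functions.
; One timeline drives Hinge1 and Hinge2 in opposite directions along X, with play rate set from separate open and close durations.
; When Looping is set, the timeline's finish triggers the opposite motion after a short delay.
; BeginPlay does nothing, so movement starts only when triggered.
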(event Custom|CloseEvent
  (Components|Timeline|SetPlayRate (Variables|Default|GetTL_OpenClose) (/ 1.0 (Variables|Default|GetClose%20Duration)))
  (bind (_direction _newtrack_0) (Timeline|TL_OpenClose Reverse)
    (:Update
      (Transformation|SetRelativeLocation (Variables|Default|GetHinge1) (Math|Vector|MakeVector (* (* _newtrack_0 2e+02) -1.0) 0.0 0.0) false false)
      (Transformation|SetRelativeLocation (Variables|Default|GetHinge2) (Math|Vector|MakeVector (* _newtrack_0 2e+02) 0.0 0.0) false false))
    (:Finished
      (if (Variables|Default|GetLooping?)
        (switch Utilities|FlowControl|Switch|SwitchonETimelineDirection _direction
          (:Forward
            (Utilities|FlowControl|Delay 0.5)
            (CallFunction|CloseEvent))
          (:Backward
            (Utilities|FlowControl|Delay 0.5)
            (CallFunction|OpenEvent)))))))

(event Custom|OpenEvent
  (Components|Timeline|SetPlayRate (Variables|Default|GetTL_OpenClose) (/ 1.0 (Variables|Default|GetOpen%20Duration)))
  (bind (_direction _newtrack_0) (Timeline|TL_OpenClose Play)
    (:Update
      (Transformation|SetRelativeLocation (Variables|Default|GetHinge1) (Math|Vector|MakeVector (* (* _newtrack_0 2e+02) -1.0) 0.0 0.0) false false)
      (Transformation|SetRelativeLocation (Variables|Default|GetHinge2) (Math|Vector|MakeVector (* _newtrack_0 2e+02) 0.0 0.0) false false))
    (:Finished
      (if (Variables|Default|GetLooping?)
        (switch Utilities|FlowControl|Switch|SwitchonETimelineDirection _direction
          (:Forward
            (Utilities|FlowControl|Delay 0.5)
            (CallFunction|CloseEvent))
          (:Backward
            (Utilities|FlowControl|Delay 0.5)
            (CallFunction|OpenEvent)))))))

(event EventBeginPlay)

(fn ConstructionScript)

(fn Open
  (CallFunction|OpenEvent))

(fn Close
  (CallFunction|CloseEvent))